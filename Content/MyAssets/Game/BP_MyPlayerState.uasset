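; Player state that syncs each player's user name and ship color to the lobby UI.
; Client update events forward to server events, which set the values and refresh the lobby widget on the first player's TwinPawn.
; OnRep handlers refresh that widget by MyPlayerID when values replicate.
; A separate server-to-multicast chain broadcasts removal of all widgets.
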(event `RemoveAllWidgets`
  ;[1 1 1] RemoveAllWidgetsClient<->Server
  (`self.ServerRemoveAllWidgets`))

(event `ServerRemoveAllWidgets`
  ;[1 1 1] RemoveAllWidgetsClient<->Server
  (`self.MultiCastRemoveAllWidgets`))

(event `MultiCastRemoveAllWidgets`
  ;[1 1 1] RemoveAllWidgetsClient<->Server
  (`WidgetLayoutLibrary.RemoveAllWidgets`))

(event `UpdateName`
  (params (Text :type Text))
  ;[1 1 1] ClientSideUserNameUpdate
  (`self.UpdateServerUserName` Text))

(event `UpdateServerUserName`
  (params (Text :type Text))
  ;[1 1 1] ServerSideUserNameUpdate
  (set `self.userName` (`KismetTextLibrary.Conv_TextToString` Text))
  (bind _astwin_pawn (cast `/Game/MyAssets/Game/TwinPawn` (`GameplayStatics.GetPlayerPawn` 0)))
  (`/Game/MyAssets/Lobby/LobbyWidget.Update Name` (`/Game/MyAssets/Game/TwinPawn.lobbyWidget` _astwin_pawn) Text (`self.myPlayerID`)))

(event `self.OnRep_UserName`
  ;[1 1 1] OnRepUserName
  (bind _astwin_pawn (cast `/Game/MyAssets/Game/TwinPawn` (`GameplayStatics.GetPlayerPawn` 0)))
  (bind _lobbywidget (`/Game/MyAssets/Game/TwinPawn.lobbyWidget` _astwin_pawn))
  (if (`KismetSystemLibrary.IsValid` _lobbywidget)
    (`/Game/MyAssets/Lobby/LobbyWidget.Update Name` _lobbywidget (`KismetTextLibrary.Conv_StringToText` (`self.userName`)) (`self.myPlayerID`))))

(event `self.OnRep_shipColor`
  ;[1 1 1] OnRepShipColor
  (bind _astwin_pawn (cast `/Game/MyAssets/Game/TwinPawn` (`GameplayStatics.GetPlayerPawn` 0)))
  (bind _lobbywidget (`/Game/MyAssets/Game/TwinPawn.lobbyWidget` _astwin_pawn))
  (if (`KismetSystemLibrary.IsValid` _lobbywidget)
    (`/Game/MyAssets/Lobby/LobbyWidget.UpdateColor` _lobbywidget (`self.myPlayerID`) (`self.shipColor`))))

(event `UpdateColor`
  (params (Color :type "LinearColor Structure"))
  ;[1 1 1] ClientSideShipColorUpdate
  (`self.ServerUpdateShipColor` Color))

(event `ServerUpdateShipColor`
  (params (Color :type "LinearColor Structure"))
  ;[1 1 1] ServerSideShipColorUpdate
  (set `self.shipColor` Color)
  (bind _astwin_pawn (cast `/Game/MyAssets/Game/TwinPawn` (`GameplayStatics.GetPlayerPawn` 0)))
  (bind _lobbywidget (`/Game/MyAssets/Game/TwinPawn.lobbyWidget` _astwin_pawn))
  (if (`KismetSystemLibrary.IsValid` _lobbywidget)
    (`/Game/MyAssets/Lobby/LobbyWidget.UpdateColor` _lobbywidget (`self.myPlayerID`) Color)))

(fn `UserConstructionScript`)